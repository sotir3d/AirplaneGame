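; Player-flown airplane pawn with thrust, pitch, roll and yaw controls, alternating guns, bomb drops and switchable cameras with orbit control.
; Thrust input drives acceleration, which decays when released and sets forward force, lift and linear damping on the Plane body each tick.
; Smoothed turn inputs rotate the actor directly.
; Flight input and tick branch on authority through Server-prefixed events, while weapon spawns and camera controls run without that routing.
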(event Custom|ServerTick
  (params (UpwardForce :type Float%20%28single-precision%29) (CurrentAcceleration :type Float%20%28single-precision%29) (MaxAcceleration :type Float%20%28single-precision%29) (CurrentRollSpeed :type Float%20%28single-precision%29) (CurrentPitchSpeed :type Float%20%28single-precision%29) (CurrentYawSpeed :type Float%20%28single-precision%29))
  (CallFunction|LocalTick UpwardForce CurrentAcceleration MaxAcceleration CurrentRollSpeed CurrentPitchSpeed CurrentYawSpeed))

(event Custom|ServerSetThrust
  (params (Thrust :type Float%20%28single-precision%29))
  (CallFunction|SetThrust Thrust))

(event Custom|SetThrust
  (params (Thrust :type Float%20%28single-precision%29))
  (bind _acceleration (Variables|Default|GetAcceleration))
  (bind _output_get (Variables|Default|SetCurrentAcceleration (Math|Float|Clamp(Float) (+ (Variables|Default|GetCurrentAcceleration) (* (Math|Float|SelectFloat (* Thrust _acceleration) (* _acceleration -0.5) (!= Thrust 0.0)) (Utilities|Time|GetWorldDeltaSeconds))) 0.0 (Variables|Default|GetMaxAcceleration))))
  (Variables|Default|SetUpwardForce (/ _output_get 1e+01)))

(event Custom|ServerChangePlaneYaw
  (params (Yaw :type Float%20%28single-precision%29))
  (CallFunction|ChangePlaneYaw Yaw))

(event Custom|LocalTick
  (params (UpwardForce :type Float%20%28single-precision%29) (CurrentAcceleration :type Float%20%28single-precision%29) (MaxAcceleration :type Float%20%28single-precision%29) (CurrentRollSpeed :type Float%20%28single-precision%29) (CurrentPitchSpeed :type Float%20%28single-precision%29) (CurrentYawSpeed :type Float%20%28single-precision%29))
  (bind _returnvalue (Utilities|Time|GetWorldDeltaSeconds))
  (Class|PrimitiveComponent|AddForceatLocationLocal (Variables|Default|GetPlane) (Math|Vector|MakeVector 0.0 0.0 UpwardForce) "200.000000, 0, 0" "None")
  (Class|PrimitiveComponent|AddForceatLocationLocal (Variables|Default|GetPlane) (Math|Vector|MakeVector 0.0 0.0 UpwardForce) "-378.000000, 0, 0" "None")
  (Class|PrimitiveComponent|AddForceatLocationLocal (Variables|Default|GetPlane) (Math|Vector|MakeVector CurrentAcceleration 0.0 0.0) "0, 0, 0" "None")
  (Class|PrimitiveComponent|SetLinearDamping (Variables|Default|GetPlane) (Math|Float|Clamp(Float) (/ CurrentAcceleration MaxAcceleration) 0.1 0.8))
  (Transformation|AddActorLocalRotation (Math|Rotator|MakeRotator (* _returnvalue CurrentRollSpeed) (* _returnvalue CurrentPitchSpeed) (* _returnvalue CurrentYawSpeed)) false false))

(event Custom|ChangePlaneYaw
  (params (Yaw :type Float%20%28single-precision%29))
  (Variables|Default|SetCurrentYawSpeed (Math|Interpolation|FInterpTo (Variables|Default|GetCurrentYawSpeed) (* Yaw (Variables|Default|GetTurnSpeed) 0.5) (Utilities|Time|GetWorldDeltaSeconds) 2.0)))

(event Custom|ServerChangePlanePitch
  (params (Pitch :type Float%20%28single-precision%29))
  (CallFunction|ChangePlanePitch Pitch))

(event Custom|ChangePlanePitch
  (params (Pitch :type Float%20%28single-precision%29))
  (Variables|Default|SetCurrentPitchSpeed (Math|Interpolation|FInterpTo (Variables|Default|GetCurrentPitchSpeed) (* Pitch (Variables|Default|GetTurnSpeed)) (Utilities|Time|GetWorldDeltaSeconds) 2.0)))

(event Custom|ServerChangePlaneRoll
  (params (Roll :type Float%20%28single-precision%29))
  (CallFunction|ChangePlaneRoll Roll))

(event Custom|ChangePlaneRoll
  (params (Roll :type Float%20%28single-precision%29))
  (Variables|Default|SetCurrentRollSpeed (Math|Interpolation|FInterpTo (Variables|Default|GetCurrentRollSpeed) (* Roll (Variables|Default|GetTurnSpeed) 2.0) (Utilities|Time|GetWorldDeltaSeconds) 2.0)))

(event EventBeginPlay)

(event Collision|EventActorBeginOverlap
  (params (OtherActor :type Actor%20Object%20Reference)))

(event EventTick
  (params (DeltaSeconds :type Float%20%28single-precision%29))
  (bind _maxacceleration (Variables|Default|GetMaxAcceleration))
  (bind _currentrollspeed (Variables|Default|GetCurrentRollSpeed))
  (bind _currentpitchspeed (Variables|Default|GetCurrentPitchSpeed))
  (bind _currentyawspeed (Variables|Default|GetCurrentYawSpeed))
  (bind _upwardforce (Variables|Default|GetUpwardForce))
  (bind _currentacceleration (Variables|Default|GetCurrentAcceleration))
  (Networking|SwitchHasAuthority
    (:Authority
      (CallFunction|LocalTick _upwardforce _currentacceleration _maxacceleration _currentrollspeed _currentpitchspeed _currentyawspeed))
    (:Remote
      (CallFunction|ServerTick _upwardforce _currentacceleration _maxacceleration _currentrollspeed _currentpitchspeed _currentyawspeed))))

(event Input|ActionEvents|InputActionFire
  (params (Key :type Key%20Structure))
  (:Pressed
    (if (Variables|Default|GetAlternateFire)
      (Game|SpawnActorfromClass "/Game/Blueprints/Projectile_BP.Projectile_BP_C" (Transformation|GetSocketTransform (Variables|Default|GetPlane) "LeftGun" "RTS_World") "Undefined" 0 0)
      (else
        (Game|SpawnActorfromClass "/Game/Blueprints/Projectile_BP.Projectile_BP_C" (Transformation|GetSocketTransform (Variables|Default|GetPlane) "RightGun" "RTS_World") "Undefined" 0 0)))
    (Variables|Default|SetAlternateFire (not (Variables|Default|GetAlternateFire)))))

(event Input|ActionEvents|InputActionSwapCamera
  (params (Key :type Key%20Structure))
  (:Pressed
    (Components|Activation|ToggleActive (Variables|Default|GetCamera))
    (Components|Activation|ToggleActive (Variables|Default|GetFPCamera))))

(event Input|ActionEvents|InputActionBomb
  (params (Key :type Key%20Structure))
  (:Pressed
    (Game|SpawnActorfromClass "/Game/Blueprints/Bomb_BP.Bomb_BP_C" (Transformation|GetSocketTransform (Variables|Default|GetPlane) "Bomb" "RTS_World") "Undefined" 0 0)))

(event Input|AxisEvents|InputAxisThrust
  (params (AxisValue :type Float%20%28single-precision%29))
  (Networking|SwitchHasAuthority
    (:Authority
      (CallFunction|SetThrust AxisValue))
    (:Remote
      (CallFunction|ServerSetThrust AxisValue))))

(event Input|AxisEvents|InputAxisPlaneRoll
  (params (AxisValue :type Float%20%28single-precision%29))
  (Networking|SwitchHasAuthority
    (:Authority
      (CallFunction|ChangePlaneRoll AxisValue))
    (:Remote
      (CallFunction|ServerChangePlaneRoll AxisValue))))

(event Input|AxisEvents|InputAxisCameraLeftRight
  (params (AxisValue :type Float%20%28single-precision%29))
  (Transformation|AddLocalRotation (Variables|Default|GetCameraStabilizer) (Math|Rotator|MakeRotator 0.0 0.0 AxisValue) false false))

(event Input|AxisEvents|InputAxisCameraUpDown
  (params (AxisValue :type Float%20%28single-precision%29))
  (bind _springarm (Variables|Default|GetSpringArm))
  (bind _returnvalue (Transformation|GetWorldRotation _springarm))
  (bind _returnvalue_2 (+ AxisValue (.pitch _returnvalue)))
  (if (and (>= _returnvalue_2 -3e+01) (<= _returnvalue_2 6e+01))
    (Transformation|AddLocalRotation (Variables|Default|GetSpringArm) (Math|Rotator|MakeRotator 0.0 AxisValue 0.0) false false)))

(event Input|AxisEvents|InputAxisPlanePitch
  (params (AxisValue :type Float%20%28single-precision%29))
  (Networking|SwitchHasAuthority
    (:Authority
      (CallFunction|ChangePlanePitch AxisValue))
    (:Remote
      (CallFunction|ServerChangePlanePitch AxisValue))))

(event Input|AxisEvents|InputAxisPlaneYaw
  (params (AxisValue :type Float%20%28single-precision%29))
  (Networking|SwitchHasAuthority
    (:Authority
      (CallFunction|ChangePlaneYaw AxisValue))
    (:Remote
      (CallFunction|ServerChangePlaneYaw AxisValue))))

(fn ConstructionScript)
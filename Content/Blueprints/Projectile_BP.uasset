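; Projectile actor that damages airplanes it overlaps.
; On BeginPlay it sets its Sphere to a custom collision object channel and starts a two-second timer that destroys the actor.
; An overlap with an actor of exactly the Airplane_BP class calls that plane's HitEvent with DamageOnHit.
; The hit does not destroy the projectile, and the graphs contain no movement logic.
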(event Custom|Destroy
  (Actor|DestroyActor))

(event EventBeginPlay
  (Utilities|Time|SetTimerbyEvent (delegate Custom|Destroy) 2.0)
  (Collision|SetCollisionObjectType (Variables|Default|GetSphere) "ECC_GameTraceChannel1"))

(event EventTick
  (params (DeltaSeconds :type Float%20%28single-precision%29)))

(event Collision|EventActorBeginOverlap
  (params (OtherActor :type Actor%20Object%20Reference))
  (if (== (Utilities|GetClass OtherActor) "/Game/Blueprints/Airplane_BP.Airplane_BP_C")
    (bind _asairplane_bp (Utilities|Casting|CastToAirplane_BP OtherActor))
    (Default|HitEvent _asairplane_bp (Variables|Default|GetDamageOnHit))))

(fn ConstructionScript)
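; Airplane game mode that runs a sequence of PlaneGoal_BP goals, activating them one at a time.
; BeginPlay gathers and counts every goal actor in the level, then activates the first.
; NextGoal increments the current index and activates that goal while the index is in range, with order taken directly from GetAllActorsOfClass.
; Nothing happens here once the last goal is passed.
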(event EventBeginPlay
  (bind _outactors (Actor|GetAllActorsOfClass "/Game/Blueprints/PlaneGoal_BP.PlaneGoal_BP_C"))
  (bind _output_get (Variables|Default|SetPlaneGoals _outactors))
  (for _array_element _output_get
    (Math|Integer|IncrementInt (Variables|Default|GetNumGoals)))
  (Default|Activate (Utilities|Array|Get(acopy) _output_get)))

(event EventTick
  (params (DeltaSeconds :type Float%20%28single-precision%29)))

(fn ConstructionScript)

(fn NextGoal
  (bind _result (Math|Integer|IncrementInt (Variables|Default|GetCurrentGoal))
    (:%20%20
      (if (< _result (Variables|Default|GetNumGoals))
        (Default|Activate (Utilities|Array|Get(acopy) (Variables|Default|GetPlaneGoals) _result))))))